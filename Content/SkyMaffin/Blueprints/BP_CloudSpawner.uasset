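; BP_CloudSpawner is an actor that procedurally spawns a rising column of BP_Cloud platforms or obstacles as BP_Muffin enters its trigger area.
; Each spawn picks a random Y within SpawnArea, moves the spawner up by SpawnSpacing and gradually shrinks cloud scale toward 1.0.
; A counter enables rain on a cloud at a set interval.
; Reset, run on BeginPlay, returns to origin, destroys existing clouds and prespawns the initial batch.
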(event OnComponentBeginOverlap(TriggerArea)
  (params (OverlappedComponent :type Primitive%20Component%20Object%20Reference) (OtherActor :type Actor%20Object%20Reference) (OtherComp :type Primitive%20Component%20Object%20Reference) (OtherBodyIndex :type Integer) (bFromSweep :type Boolean) (SweepResult :type Hit%20Result%20Structure%20%28by%20ref%29))
  (Utilities|Casting|CastToBP_Muffin OtherActor)
  (CallFunction|SpawnCloud))

(event EventBeginPlay
  (CallFunction|Reset))

(fn ConstructionScript)

(fn SpawnCloud
  (bind _spawnarea (Variables|Default|GetSpawnArea))
  (bind _returnvalue (Transformation|GetWorldLocation _spawnarea))
  (bind (_origin _boxextent) (Collision|GetComponentBounds _spawnarea))
  (Utilities|FlowControl|Sequence
    (:then_0
      (bind _returnvalue_2 (Game|SpawnActorfromClass "/Game/SkyMaffin/Blueprints/BP_Cloud.BP_Cloud_C" (Math|Transform|MakeTransform (Math|Vector|MakeVector (.x _returnvalue) (.y (Math|Random|RandomPointinBoundingBox _origin _boxextent)) (.z _returnvalue)) "0, 0, 0" (Math|Conversions|ToVector(Float) (Variables|Default|GetSpawnScale))) "Undefined" 0 0))
      (LocalVariables|SetCloud _returnvalue_2))
    (:then_1
      (Transformation|AddActorWorldOffset (Math|Vector|MakeVector 0.0 0.0 (Variables|Default|GetSpawnSpacing)))
      (if (> (Variables|Default|GetSpawnScale) 1.0)
        (Variables|Default|SetSpawnScale (- (Variables|Default|GetSpawnScale) 0.01))))
    (:then_2
      (Math|Integer|IncrementInt (Variables|Default|GetSpawnsSinceLastRainCloud)
        (:%20%20
          (if (>= (Variables|Default|GetSpawnsSinceLastRainCloud) (Variables|Default|GetRainCloudSpawnInterval))
            (Default|EnableRain (LocalVariables|GetCloud))
            (Variables|Default|SetSpawnsSinceLastRainCloud 0)))))))

(fn Reset
  (Utilities|FlowControl|Sequence
    (:then_0
      (Variables|Default|SetSpawnScale (Variables|Default|GetSpawnInitialScale))
      (Variables|Default|SetSpawnsSinceLastRainCloud 0))
    (:then_1
      (Transformation|SetActorLocation "0, 0, 0" false false))
    (:then_2
      (bind _outactors (Actor|GetAllActorsOfClass "/Game/SkyMaffin/Blueprints/BP_Cloud.BP_Cloud_C"))
      (for _array_element _outactors
        (Actor|DestroyActor _array_element)))
    (:then_3
      (for _index (range 0 (- (Variables|Default|GetInitialSpawnAmount) 1))
        (CallFunction|SpawnCloud)))))